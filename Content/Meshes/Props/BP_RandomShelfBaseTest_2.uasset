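; BP_RandomShelfBaseTest_2 is a test shelf prop that randomly fills itself with static meshes at construction time.
; The construction script sets the base mesh, then loops over an X by Z grid of evenly spaced slots from an origin.
; Each slot rolls a weighted chance, then adds a uniformly scaled, static-mobility component with a mesh picked at random from a list.
; It uses unseeded randomness and has no active runtime logic.
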(event EventBeginPlay)

(event Collision|EventActorBeginOverlap
  (params (OtherActor :type Actor%20Object%20Reference)))

(event EventTick
  (params (DeltaSeconds :type Float%20%28single-precision%29)))

(fn ConstructionScript
  (Components|StaticMesh|SetStaticMesh (Variables|Default|GetMesh) (Variables|Default|GetNew%20Mesh))
  (for _index (range 0 (- (Variables|Default|GetNumOfMeshesX) 1))
    (for _index_2 (range 0 (- (Variables|Default|GetNumOfMeshesY) 1))
      (if (Math|Random|RandomBoolwithWeight (Variables|Default|GetChanceToSpawn))
        (bind _returnvalue (AddComponent|AddStaticMeshComponent false (Math|Transform|MakeTransform (+ (Variables|Default|GetOrigin) (Math|Vector|MakeVector (* _index (Variables|Default|GetHorizontalSpacing)) 0.0 (* _index_2 (Variables|Default|GetVerticalSpacing)))) "0, 0, 0" (Math|Conversions|ToVector(Float) (Variables|Default|GetMeshScale)))))
        (Components|StaticMesh|SetStaticMesh _returnvalue (.OutItem (Utilities|Array|Random (Variables|Default|GetMeshesToSpawn))))
        (Transformation|SetMobility _returnvalue "Static")))))