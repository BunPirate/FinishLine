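; BP_MenuPawn is the main menu pawn, which eases between a default pose and an offset pose.
; The Offset and Reset events set a boolean that selects the target location and rotation.
; Tick interpolates the actor toward that target with VInterpTo and RInterpTo, using absolute transforms, so the default pose is the world origin with zero rotation.
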(event Custom|Reset
  (Variables|Default|SetOffset? false))

(event Custom|Offset
  (Variables|Default|SetOffset? true))

(event EventTick
  (params (DeltaSeconds :type Float%20%28single-precision%29))
  (bind _offset_ (Variables|Default|GetOffset?))
  (Transformation|SetActorRotation (Math|Interpolation|RInterpTo (Transformation|GetActorRotation) (Math|Rotator|SelectRotator "15.000000,-15.000000, 0" "0, 0, 0" _offset_) DeltaSeconds 1.0))
  (Transformation|SetActorLocation (Math|Interpolation|VInterpTo (Transformation|GetActorLocation) (Math|Vector|SelectVector "-100.000000, 0, 0" "0.000000, 0, 0" _offset_) DeltaSeconds 1.0) false false))

(fn ConstructionScript)