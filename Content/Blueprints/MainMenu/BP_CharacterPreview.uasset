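; BP_CharacterPreview is a main menu preview actor whose skeletal mesh tilts in response to the mouse cursor.
; Each Tick, it traces under the cursor and takes the pitch of the direction from the hit point to the actor.
; That pitch is smoothed with RInterpTo and applied as the mesh's relative roll, with pitch and yaw held at zero.
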(event EventBeginPlay
  (Variables|Default|SetControllerRef (Class|GameplayStatics|GetPlayerControllerfromID)))

(event EventTick
  (params (DeltaSeconds :type Float%20%28single-precision%29))
  (bind _controllerref (Variables|Default|GetControllerRef))
  (bind _hitresult (Game|Player|GetHitResultUnderCursorbyChannel _controllerref "TraceTypeQuery1" true))
  (Utilities|IsValid _controllerref
    (:Is%20Valid
      (if (.bblockinghit _hitresult)
        (Transformation|SetRelativeRotation (Variables|Default|GetSkeletalMesh) (Math|Rotator|MakeRotator (.roll (Math|Interpolation|RInterpTo (Math|Rotator|MakeRotator (Variables|Default|GetCurrentRot) 0.0 0.0) (Math|Rotator|MakeRotator (.pitch (Math|Conversions|RotationFromXVector (Math|Vector|GetUnitDirection(Vector) (.location _hitresult) (Transformation|GetActorLocation)))) 0.0 0.0) (Utilities|Time|GetWorldDeltaSeconds) 5.0)) 0.0 0.0) false false)
        (Variables|Default|SetCurrentRot (.roll (Math|Interpolation|RInterpTo (Math|Rotator|MakeRotator (Variables|Default|GetCurrentRot) 0.0 0.0) (Math|Rotator|MakeRotator (.pitch (Math|Conversions|RotationFromXVector (Math|Vector|GetUnitDirection(Vector) (.location _hitresult) (Transformation|GetActorLocation)))) 0.0 0.0) (Utilities|Time|GetWorldDeltaSeconds) 5.0)))))))

(fn ConstructionScript)