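; Throwable homing rocket item that chases the nearest player-interface actor and explodes on impact.
; When thrown, it enables physics and adds a homing projectile movement component, then re-targets every tick while not held.
; The first hit fires a radial impulse, effects and distance-scaled damage to sphere overlaps, then destroys the rocket.
; A helper function estimates its distance along an AI path spline.
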(event OnComponentHit(Hitbox)
  (params (HitComponent :type Primitive%20Component%20Object%20Reference) (OtherActor :type Actor%20Object%20Reference) (OtherComp :type Primitive%20Component%20Object%20Reference) (NormalImpulse :type Vector :default "0, 0, 0") (Hit :type Hit%20Result%20Structure%20%28by%20ref%29))
  (bind _returnvalue (Transformation|GetActorLocation))
  (if (not (Variables|Default|GetHeldByPlayer))
    (Utilities|FlowControl|DoOnce false
      (:Completed
        (Class|RadialForceComponent|FireImpulse (Variables|Default|GetExplosionForce))
        (Niagara|SpawnSystematLocation "/Game/NiagaraSystems/NS_RocketExplosion.NS_RocketExplosion" _returnvalue)
        (Audio|PlaySoundatLocation "/Game/Audio/SFX/Obsticles/Flip_Controls_SFX.Flip_Controls_SFX" _returnvalue "0, 0, 0" 1.0 1.0 0.0 "/Game/Audio/SoundAttenuation.SoundAttenuation" "/Game/Audio/SoundConcurrency.SoundConcurrency" 0 0)
        (for _array_element (Collision|GetOverlappingActors (Variables|Default|GetSphere) 0 :!class /Script/Engine.PrimitiveComponent)
          (Class|BPIDamageable|DoDamage(Message) _array_element (Math|Float|Truncate (Math|Float|Lerp 3e+02 0.0 (Math|Float|MapRangeClamped (Transformation|GetDistanceTo _array_element) 0.0 1e+03 1.0 0.0)))))
        (Actor|DestroyActor)))))

(event EventTick
  (params (DeltaSeconds :type Float%20%28single-precision%29))
  (bind _projectilecomponent (Variables|Default|GetProjectileComponent))
  (if (not (Variables|Default|GetHeldByPlayer))
    (Variables|Default|SetClosestDistance 1e+08)
    (bind _outactors (Actor|GetAllActorswithInterface "/Game/Blueprints/Interfaces/BPI_Player.BPI_Player_C"))
    (for _array_element _outactors
      (if (and (not (== _array_element self)) (< (Transformation|GetDistanceTo _array_element) (Variables|Default|GetClosestDistance)))
        (Variables|Default|SetClosestDistance (Transformation|GetDistanceTo _array_element))
        (Variables|Default|SetCurrentTarget _array_element)))
    (bind _playerref (Class|BPIPlayer|GetPlayer(Message) (Variables|Default|GetCurrentTarget)))
    (Utilities|IsValid _playerref
      (:Is%20Valid
        (Variables|/Script/Engine.ProjectileMovementComponent|SetHomingTargetComponent _projectilecomponent (Variables|/Script/Engine.Actor|GetRootComponent _playerref))
        (Development|PrintString (Utilities|GetDisplayName (Variables|/Script/Engine.ProjectileMovementComponent|GetHomingTargetComponent _projectilecomponent)))))))

(event EventThrown
  (Variables|Default|SetHeldByPlayer false)
  (Components|Activation|Activate (Variables|Default|GetTrail) false)
  (Physics|SetSimulatePhysics (Variables|Default|GetHitbox) true)
  (bind _returnvalue (AddComponent|AddProjectileMovementComponent))
  (Variables|/Script/Engine.ProjectileMovementComponent|SetbIsHomingProjectile _returnvalue true)
  (Variables|/Script/Engine.ProjectileMovementComponent|SetHomingAccelerationMagnitude _returnvalue 2.5e+04)
  (Variables|Default|SetProjectileComponent _returnvalue)
  (Variables|Default|SetClosestDistance 1e+08)
  (bind _outactors (Actor|GetAllActorswithInterface "/Game/Blueprints/Interfaces/BPI_Player.BPI_Player_C"))
  (for _array_element _outactors
    (if (and (not (== _array_element self)) (< (Transformation|GetDistanceTo _array_element) (Variables|Default|GetClosestDistance)))
      (Variables|Default|SetClosestDistance (Transformation|GetDistanceTo _array_element))
      (Variables|Default|SetCurrentTarget _array_element)))
  (bind _playerref (Class|BPIPlayer|GetPlayer(Message) (Variables|Default|GetCurrentTarget)))
  (Utilities|IsValid _playerref
    (:Is%20Valid
      (Variables|/Script/Engine.ProjectileMovementComponent|SetHomingTargetComponent (Variables|Default|GetProjectileComponent) (Variables|/Script/Engine.Actor|GetRootComponent _playerref))
      (Development|PrintString (Utilities|GetDisplayName (Variables|/Script/Engine.ProjectileMovementComponent|GetHomingTargetComponent (Variables|Default|GetProjectileComponent)))))))

(fn ConstructionScript
  (|CallParentFunction))

(fn DistanceAlongPath
  (params (AIPathRef :type BP%20AI%20Path%20Object%20Reference))
  (bind _returnvalue (Transformation|GetActorLocation))
  (bind _spline (Variables|/Game/Blueprints/AI/BP_AIPath.BP_AIPath_C|GetSpline AIPathRef))
  (bind _returnvalue_2 (Class|SplineComponent|FindInputKeyClosesttoWorldLocation _spline _returnvalue))
  (bind _returnvalue_3 (Math|Float|Truncate _returnvalue_2))
  (bind _returnvalue_4 (+ _returnvalue_3 1))
  (LocalVariables|SetPrev%20Location (Spline|GetLocationatSplinePoint _spline _returnvalue_3 "World"))
  (LocalVariables|SetNext%20Location (Spline|GetLocationatSplinePoint _spline _returnvalue_4 "World"))
  (return (Math|Float|Lerp (Spline|GetDistanceAlongSplineatSplinePoint _spline _returnvalue_3) (Spline|GetDistanceAlongSplineatSplinePoint _spline _returnvalue_4) (/ (Math|Vector|VectorLength (- (Spline|FindLocationClosesttoWorldLocation _spline (Transformation|GetActorLocation) "World") (LocalVariables|GetPrev%20Location))) (Math|Vector|VectorLength (- (LocalVariables|GetNext%20Location) (LocalVariables|GetPrev%20Location)))))))