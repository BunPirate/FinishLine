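; BP_ThrowableSlime is a throwable item that becomes a slime puddle slowing players on overlap.
; On its first hit while not held, it destroys itself if overlapping another throwable; otherwise it enables itself and disables physics and collision on its hitbox.
; A downward trace aligns it to the surface normal, then a timeline expands mesh and decal.
; Once enabled, SlowCollision overlaps apply and clear a high-friction effect through player messages.
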(event OnComponentBeginOverlap(SlowCollision)
  (params (OverlappedComponent :type Primitive%20Component%20Object%20Reference) (OtherActor :type Actor%20Object%20Reference) (OtherComp :type Primitive%20Component%20Object%20Reference) (OtherBodyIndex :type Integer) (bFromSweep :type Boolean) (SweepResult :type Hit%20Result%20Structure%20%28by%20ref%29))
  (if (Variables|Default|GetEnabled?)
    (bind _playerref (Class|BPIPlayer|GetPlayer(Message) OtherActor))
    (Utilities|IsValid _playerref
      (:Is%20Valid
        (Default|HighFrictionEffect _playerref 3.0)))))

(event OnComponentHit(Hitbox)
  (params (HitComponent :type Primitive%20Component%20Object%20Reference) (OtherActor :type Actor%20Object%20Reference) (OtherComp :type Primitive%20Component%20Object%20Reference) (NormalImpulse :type Vector :default "0, 0, 0") (Hit :type Hit%20Result%20Structure%20%28by%20ref%29))
  (bind _returnvalue (Transformation|GetActorLocation))
  (bind _hitbox (Variables|Default|GetHitbox))
  (if (not (Variables|Default|GetHeldByPlayer))
    (Utilities|FlowControl|DoOnce false
      (:Completed
        (for _array_element (Collision|GetOverlappingActors (Variables|Default|GetAreaCheck) "/Game/Blueprints/ItemObstacles/BP_ThrowableBase.BP_ThrowableBase_C" :!class /Script/Engine.PrimitiveComponent)
          (bind _throwableref (Class|BPIThrowable|GetThrowable(Message) _array_element))
          (Utilities|IsValid _throwableref
            (:Is%20Valid
              (if (not (== _throwableref self))
                (Variables|Default|SetOverlappingWithOtherThrowable true)))))
        (if (Variables|Default|GetOverlappingWithOtherThrowable)
          (Actor|DestroyActor)
          (else
            (Variables|Default|SetEnabled? true)
            (Physics|SetSimulatePhysics _hitbox false)
            (Collision|SetCollisionEnabled _hitbox "NoCollision")
            (bind _outhit (Collision|LineTraceByChannel _returnvalue (- _returnvalue "0,0,250.000000") "TraceTypeQuery1" false 0 "None"))
            (Transformation|SetActorRotation (Math|Rotator|MakeRotator (.roll (Math|Conversions|RotationFromXVector (Math|Vector|RotateVectorAroundAxis (.Normal (Collision|BreakHitResult _outhit)) -9e+01 "1.000000, 0, 0"))) (.pitch (Math|Conversions|RotationFromXVector (Math|Vector|RotateVectorAroundAxis (.Normal (Collision|BreakHitResult _outhit)) -9e+01 "1.000000, 0, 0"))) (.yaw (Transformation|GetActorRotation))))
            ;[1 1 1] Sound
            (Audio|PlaySoundatLocation "/Engine/VREditor/Sounds/UI/Dockable_Window_Open.Dockable_Window_Open" (Transformation|GetActorLocation) "0, 0, 0" 1.0 1.0 0.0 "/Game/Audio/SoundAttenuation.SoundAttenuation" "/Game/Audio/SoundConcurrency.SoundConcurrency" 0 0)
            (Components|DestroyComponent (Variables|Default|GetCube))
            ;[1 1 1] Expand
            (bind _lerp (Timeline|Timeline_0 Play)
              (:Update
                (Transformation|SetRelativeScale3D (Variables|Default|GetMeshParent) (Math|Vector|Lerp(Vector) "1.000000,1.000000,1.000000" "10.000000,10.000000,2.500000" _lerp))
                (Transformation|SetRelativeScale3D (Variables|Default|GetDecal) (Math|Vector|MakeVector 0.5 (.Y (Math|Vector|BreakVector (Math|Vector|Lerp(Vector) "1.000000,1.000000,1.000000" "10.000000,10.000000,2.500000" _lerp))) (.X (Math|Vector|BreakVector (Math|Vector|Lerp(Vector) "1.000000,1.000000,1.000000" "10.000000,10.000000,2.500000" _lerp)))))))))))))

(event OnComponentEndOverlap(SlowCollision)
  (params (OverlappedComponent :type Primitive%20Component%20Object%20Reference) (OtherActor :type Actor%20Object%20Reference) (OtherComp :type Primitive%20Component%20Object%20Reference) (OtherBodyIndex :type Integer))
  (if (Variables|Default|GetEnabled?)
    (bind _playerref (Class|BPIPlayer|GetPlayer(Message) OtherActor))
    (Utilities|IsValid _playerref
      (:Is%20Valid
        (Default|ClearHighFrictionEffect _playerref)))))

(fn ConstructionScript
  (|CallParentFunction))