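; BP_ThrowableBase is the base actor for throwable items that deploy once, on their first hit after leaving the player's hands.
; On that hit, an area check looks for overlapping actors of exactly the base class and calls PutBackInInventory, which here only destroys the actor.
; Otherwise it enables itself, turns off hitbox physics and collision, tilts to a downward trace's surface normal, and grows its mesh through the Expand timeline.
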(event OnComponentHit(Hitbox)
  (params (HitComponent :type Primitive%20Component%20Object%20Reference) (OtherActor :type Actor%20Object%20Reference) (OtherComp :type Primitive%20Component%20Object%20Reference) (NormalImpulse :type Vector :default "0, 0, 0") (Hit :type Hit%20Result%20Structure%20%28by%20ref%29))
  (bind _returnvalue (Transformation|GetActorLocation))
  (bind _hitbox (Variables|Default|GetHitbox))
  (if (not (Variables|Default|GetHeldByPlayer))
    (Utilities|FlowControl|DoOnce false
      (:Completed
        (for _array_element (Collision|GetOverlappingActors (Variables|Default|GetAreaCheck) "BP_ThrowableBase_C" :!class /Script/Engine.PrimitiveComponent)
          (if (== (Utilities|GetClass _array_element) "BP_ThrowableBase_C")
            (Variables|Default|SetOverlappingWithOtherThrowable true)))
        (if (Variables|Default|GetOverlappingWithOtherThrowable)
          (CallFunction|PutBackinInventory)
          (else
            (Variables|Default|SetEnabled? true)
            (Physics|SetSimulatePhysics _hitbox false)
            (Collision|SetCollisionEnabled _hitbox "NoCollision")
            (bind _outhit (Collision|LineTraceByChannel _returnvalue (- _returnvalue "0,0,250.000000") "TraceTypeQuery1" false 0 "None"))
            (Transformation|SetActorRotation (Math|Rotator|MakeRotator (.roll (Math|Conversions|RotationFromXVector (Math|Vector|RotateVectorAroundAxis (.Normal (Collision|BreakHitResult _outhit)) -9e+01 "1.000000, 0, 0"))) (.pitch (Math|Conversions|RotationFromXVector (Math|Vector|RotateVectorAroundAxis (.Normal (Collision|BreakHitResult _outhit)) -9e+01 "1.000000, 0, 0"))) (.yaw (Transformation|GetActorRotation))))
            (bind _lerp (Timeline|Expand Play)
              (:Update
                (Transformation|SetRelativeScale3D (Variables|Default|GetMeshParent) (Math|Vector|Lerp(Vector) "0.250000,0.250000,0.250000" "1.000000,1.000000,1.000000" _lerp))))))))))

(event Custom|PutBackInInventory
  (Actor|DestroyActor))

(fn ConstructionScript)

(fn GetThrowable
  (return self))