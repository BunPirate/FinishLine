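; BP_SoapPuddle is a slippery floor obstacle that affects players while they stand in it.
; Overlapping its box calls SlipperyEffect on the actor's PlayerMessage, and leaving calls ClearSlipperyEffect.
; Entry also plays an attenuated splash sound, throttled by a DoOnce that resets after a short delay.
; The construction script sizes the box and decal from one Size variable.
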(event OnComponentBeginOverlap(OverlapBox)
  (params (OverlappedComponent :type Primitive%20Component%20Object%20Reference) (OtherActor :type Actor%20Object%20Reference) (OtherComp :type Primitive%20Component%20Object%20Reference) (OtherBodyIndex :type Integer) (bFromSweep :type Boolean) (SweepResult :type Hit%20Result%20Structure%20%28by%20ref%29))
  (bind _playerref (Class|BPIPlayer|GetPlayer(Message) OtherActor))
  (Utilities|IsValid _playerref
    (:Is%20Valid
      (Default|SlipperyEffect _playerref)
      (Utilities|FlowControl|DoOnce false :!label _label
        (:Completed
          (Audio|PlaySoundatLocation "/Game/Audio/SFX/Obsticles/Soap_Puddle_SFX.Soap_Puddle_SFX" (Transformation|GetActorLocation) "0, 0, 0" 1.0 1.0 0.0 "/Game/Audio/SoundAttenuation.SoundAttenuation" 0 0 0)
          (Utilities|FlowControl|Delay 0.5)
          (goto _label Reset))))))

(event OnComponentEndOverlap(OverlapBox)
  (params (OverlappedComponent :type Primitive%20Component%20Object%20Reference) (OtherActor :type Actor%20Object%20Reference) (OtherComp :type Primitive%20Component%20Object%20Reference) (OtherBodyIndex :type Integer))
  (bind _playerref (Class|BPIPlayer|GetPlayer(Message) OtherActor))
  (Utilities|IsValid _playerref
    (:Is%20Valid
      (Default|ClearSlipperyEffect _playerref))))

(fn ConstructionScript
  (bind _size (Variables|Default|GetSize))
  (bind _returnvalue (/ _size 1e+02))
  (bind (_x _y) (Math|Vector|BreakVector _returnvalue))
  (Components|Box|SetBoxExtent (Variables|Default|GetOverlapBox) _size true)
  (Transformation|SetRelativeScale3D (Variables|Default|GetDecal) (Math|Vector|MakeVector 1.0 _y _x)))