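; Falling treat obstacle that damages and launches the player on impact.
; On spawn, a timeline scales up a decal as the treat's marker.
; On a collision hit, interface messages fetch the player and apply damage, followed by an upward velocity-change impulse on the player's body.
; Any hit, player or not, spawns a Niagara breaking effect and destroys the treat.
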(event OnComponentHit(Collision)
  (params (HitComponent :type Primitive%20Component%20Object%20Reference) (OtherActor :type Actor%20Object%20Reference) (OtherComp :type Primitive%20Component%20Object%20Reference) (NormalImpulse :type Vector :default "0, 0, 0") (Hit :type Hit%20Result%20Structure%20%28by%20ref%29))
  (bind _playerref (Class|BPIPlayer|GetPlayer(Message) OtherActor))
  (Utilities|IsValid _playerref
    (:Is%20Valid
      (bind _output_get (Variables|Default|SetPlayer%20Ref _playerref))
      (Class|BPIDamageable|DoDamage(Message) _output_get (Variables|Default|GetTreatDamage) self)
      (Physics|AddImpulse (Variables|/Game/Blueprints/Player/BP_CustomVehicle.BP_CustomVehicle_C|GetBody (Variables|Default|GetPlayer%20Ref)) "0, 0,1000.000000" "None" true))
    (:Is%20Not%20Valid
      _))
  ;[1 1 1] Treat breaking effect
  (Niagara|SpawnSystematLocation "/Game/NiagaraSystems/NS_Pickup.NS_Pickup" (Transformation|GetActorLocation))
  (Actor|DestroyActor))

(event EventBeginPlay
  (bind _decalsize (Timeline|DecalSize Play)
    (:Update
      (Transformation|SetRelativeScale3D (Variables|Default|GetDecal) (Math|Vector|MakeVector 1.0 (Math|Float|Lerp 0.01 0.15 _decalsize) (Math|Float|Lerp 0.01 0.15 _decalsize))))))

(fn ConstructionScript)