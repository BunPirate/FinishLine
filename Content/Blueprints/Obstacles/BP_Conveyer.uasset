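; BP_Conveyer is a conveyor obstacle that pushes player actors along the forward vector of its Direction component.
; Each Tick it checks actors overlapping CollisionBox, keeps those returning a valid GetPlayerMessage result, and applies a swept world offset scaled by Speed and delta time.
; The construction script derives the box extent and the mesh's X/Y scale from Size, keeping mesh height fixed.
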(event EventBeginPlay)

(event Collision|EventActorBeginOverlap
  (params (OtherActor :type Actor%20Object%20Reference)))

(event EventTick
  (params (DeltaSeconds :type Float%20%28single-precision%29))
  (for _array_element (Collision|GetOverlappingActors (Variables|Default|GetCollisionBox) 0 :!class /Script/Engine.PrimitiveComponent)
    (bind _playerref (Class|BPIPlayer|GetPlayer(Message) _array_element))
    (Utilities|IsValid _playerref
      (:Is%20Valid
        (Transformation|AddActorWorldOffset _array_element (* (Math|Vector|GetForwardVector (Transformation|GetWorldRotation (Variables|Default|GetDirection))) (* DeltaSeconds (Variables|Default|GetSpeed))) true true)))))

(fn ConstructionScript
  (bind _size (Variables|Default|GetSize))
  (bind _returnvalue (/ _size 5e+01))
  (Components|Box|SetBoxExtent (Variables|Default|GetCollisionBox) _size true)
  (Transformation|SetRelativeScale3D (Variables|Default|GetMesh) (Math|Vector|MakeVector (.x _returnvalue) (.y _returnvalue) 0.25)))