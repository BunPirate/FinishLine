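; BP_LeakedBag is an obstacle: a leaking bag whose growing food spill applies a high-friction effect to the player.
; On BeginPlay, the Growth timeline scales OriginPoint from StartSize to Maxsize, then deactivates the NSTreatFalling effect.
; FoodMesh overlaps fetch the player through GetPlayerMessage to apply or clear the effect; older direct Speed edits are disconnected.
; The construction script previews the maximum spill size and sets the bag height.
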(event OnComponentBeginOverlap(FoodMesh)
  (params (OverlappedComponent :type Primitive%20Component%20Object%20Reference) (OtherActor :type Actor%20Object%20Reference) (OtherComp :type Primitive%20Component%20Object%20Reference) (OtherBodyIndex :type Integer) (bFromSweep :type Boolean) (SweepResult :type Hit%20Result%20Structure%20%28by%20ref%29))
  (bind _playerref (Class|BPIPlayer|GetPlayer(Message) OtherActor))
  (Utilities|IsValid _playerref
    (:Is%20Valid
      (bind _output_get (Variables|Default|SetPlayer%20Ref _playerref))
      (Default|HighFrictionEffect _output_get))))

(event OnComponentEndOverlap(FoodMesh)
  (params (OverlappedComponent :type Primitive%20Component%20Object%20Reference) (OtherActor :type Actor%20Object%20Reference) (OtherComp :type Primitive%20Component%20Object%20Reference) (OtherBodyIndex :type Integer))
  (bind _playerref (Class|BPIPlayer|GetPlayer(Message) OtherActor))
  (Utilities|IsValid _playerref
    (:Is%20Valid
      (bind _output_get (Variables|Default|SetPlayer%20Ref _playerref))
      (Default|ClearHighFrictionEffect _output_get))))

(event EventBeginPlay
  (Components|Timeline|SetPlayRate (Variables|Default|GetGrowth) (Variables|Default|GetPlayRate))
  (bind _growth (Timeline|Growth Play)
    (:Update
      (Transformation|SetRelativeScale3D (Variables|Default|GetOriginPoint) (Math|Conversions|ToVector(Float) (Math|Float|Lerp (Variables|Default|GetStartSize) (Variables|Default|Getmaxsize) _growth))))
    (:Finished
      (Components|Activation|Deactivate (Variables|Default|GetNS_TreatFalling)))))

(fn ConstructionScript
  (bind _bag (Variables|Default|GetBag))
  (bind _relativelocation (Variables|/Script/Engine.SceneComponent|GetRelativeLocation _bag))
  (Transformation|SetRelativeScale3D (Variables|Default|GetFoodMeshPreview) (Math|Conversions|ToVector(Float) (Variables|Default|Getmaxsize)))
  (Transformation|SetRelativeLocation _bag (Math|Vector|MakeVector (.x _relativelocation) (.y _relativelocation) (Variables|Default|GetBagHeight)) false false))