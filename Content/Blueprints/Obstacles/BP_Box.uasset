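; BP_Box is a destructible obstacle box that loses health when it receives a DoDamage event.
; DoDamage passes the damage to HealthUpdate, which adds or subtracts an amount and clamps CurrentHealth between zero and MaxHealth.
; At zero health the box spawns an enlarged NS_Pickup Niagara effect at its location and destroys itself.
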(event EventBeginPlay)

(event EventDoDamage
  (params (Damage :type Integer) (Instigator :type Actor%20Object%20Reference))
  (CallFunction|HealthUpdate (Math|Conversions|ToFloat(Integer) Damage) false)
  (if (<= (Variables|Default|GetCurrentHealth) 0.0)
    (Niagara|SpawnSystematLocation "/Game/NiagaraSystems/NS_Pickup.NS_Pickup" (Transformation|GetActorLocation) "0, 0, 0" "10.000000,10.000000,10.000000")
    (Actor|DestroyActor)))

(fn ConstructionScript)

(fn HealthUpdate
  (params (Amount :type Float%20%28double-precision%29) (Positive :type Boolean))
  (LocalVariables|SetL_Health (Variables|Default|GetCurrentHealth))
  (if Positive
    ;[1 1 1] +health
    (LocalVariables|SetL_Health (+ (LocalVariables|GetL_Health) Amount))
    (else
      ;[1 1 1] -health
      (LocalVariables|SetL_Health (- (LocalVariables|GetL_Health) Amount))))
  (bind _output_get (LocalVariables|SetL_Health (Math|Float|Clamp(Float) (LocalVariables|GetL_Health) 0.0 (Variables|Default|GetMaxHealth))))
  (Variables|Default|SetCurrentHealth _output_get))