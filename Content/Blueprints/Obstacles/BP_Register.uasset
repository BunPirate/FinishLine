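; BP_Register is an obstacle that repeatedly shakes as a tell and then pops its static mesh out along the X axis.
; BeginPlay starts a looping timer on a configurable delay to trigger each cycle.
; A Shaking timeline offsets the mesh's relative location, then after a short pause a PopOut2 timeline drives the pop, each scaled by its own distance variable without sweeping.
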(event Custom|Pop-Out
  (bind _alpha (Timeline|Shaking PlayFromStart)
    (:Update
      (Transformation|SetRelativeLocation (Variables|Default|GetStaticMesh) (* (* _alpha "1.000000,0,0") (Variables|Default|GetShakingDistance)) false false))
    (:Finished
      (Utilities|FlowControl|Delay 0.5)
      (bind _alpha_2 (Timeline|PopOut PlayFromStart)
        (:Update
          (Transformation|SetRelativeLocation (Variables|Default|GetStaticMesh) (* (* _alpha_2 "1.000000,0,0") (Variables|Default|GetPop-OutDistance)) false false))))))

(event EventBeginPlay
  (Utilities|Time|SetTimerbyEvent (delegate Custom|Pop-Out) (Variables|Default|GetDelay) true))

(fn ConstructionScript)

(fn NewFunction0)