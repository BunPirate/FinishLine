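; A high-friction obstacle area, shown as a doormat, that affects players who step onto it.
; Overlapping the hitbox gets the actor's PlayerMessage and, if valid, applies the high-friction effect, then clears it when the overlap ends.
; The construction script gives the visible mat and hitbox the same configurable mesh and horizontal scale, with the hitbox stretched taller in Z.
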(event OnComponentBeginOverlap(DoormatHitbox)
  (params (OverlappedComponent :type Primitive%20Component%20Object%20Reference) (OtherActor :type Actor%20Object%20Reference) (OtherComp :type Primitive%20Component%20Object%20Reference) (OtherBodyIndex :type Integer) (bFromSweep :type Boolean) (SweepResult :type Hit%20Result%20Structure%20%28by%20ref%29))
  (bind _playerref (Class|BPIPlayer|GetPlayer(Message) OtherActor))
  (Utilities|IsValid _playerref
    (:Is%20Valid
      (Default|HighFrictionEffect _playerref))))

(event OnComponentEndOverlap(DoormatHitbox)
  (params (OverlappedComponent :type Primitive%20Component%20Object%20Reference) (OtherActor :type Actor%20Object%20Reference) (OtherComp :type Primitive%20Component%20Object%20Reference) (OtherBodyIndex :type Integer))
  (bind _playerref (Class|BPIPlayer|GetPlayer(Message) OtherActor))
  (Utilities|IsValid _playerref
    (:Is%20Valid
      (Default|ClearHighFrictionEffect _playerref))))

(fn ConstructionScript
  (bind _mesh (Variables|Default|GetMesh))
  (bind _scale (Variables|Default|GetScale))
  (bind _scale_2 (Variables|Default|GetScale))
  (Components|StaticMesh|SetStaticMesh (Variables|Default|GetDoormat) _mesh)
  (Components|StaticMesh|SetStaticMesh (Variables|Default|GetDoormatHitbox) _mesh)
  (Transformation|SetRelativeScale3D (Variables|Default|GetDoormat) (Math|Vector|MakeVector _scale_2 _scale_2 1.0))
  (Transformation|SetRelativeScale3D (Variables|Default|GetDoormatHitbox) (Math|Vector|MakeVector _scale _scale 5.0)))