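; BP_MovingBall is a rolling obstacle that damages and knocks back player vehicles.
; Each cycle picks a random mesh and uses the MoveBall timeline to move and rotate the ball from its start toward a target offset, then resets and repeats after a delay.
; Colliding with a vehicle, identified by an interface message, stops the timeline, deals damage, plays a montage, launches the vehicle along the ball's forward vector and restarts the cycle.
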(event OnComponentHit(SphereCollision)
  (params (HitComponent :type Primitive%20Component%20Object%20Reference) (OtherActor :type Actor%20Object%20Reference) (OtherComp :type Primitive%20Component%20Object%20Reference) (NormalImpulse :type Vector :default "0, 0, 0") (Hit :type Hit%20Result%20Structure%20%28by%20ref%29))
  (bind _playerref (Class|BPIPlayer|GetPlayer(Message) OtherActor))
  (Utilities|IsValid _playerref
    (:Is%20Valid
      (Variables|Default|SetAs%20BP%20Vehicle%20Base _playerref)
      (CallFunction|Hit)
      (Class|BPIDamageable|DoDamage(Message) (Variables|Default|GetAs%20BP%20Vehicle%20Base) (Variables|Default|GetDamage) self)
      ;[1 1 1] Animtion when ball is hit
      (Animation|Montage|PlayMontage 0 0
        (:then
          (Physics|AddImpulse (Variables|/Script/ChaosVehicles.WheeledVehiclePawn|GetMesh (Variables|Default|GetAs%20BP%20Vehicle%20Base)) (* (Transformation|GetActorForwardVector) 5e+03) "None" true)
          ;[1 1 1] (Should be on complete anim)
          (Transformation|SetWorldLocation (Variables|Default|GetDefaultSceneRoot) (Variables|Default|GetStartLocation) false false)
          (Utilities|FlowControl|Delay (Variables|Default|GetWaitTime))
          (CallFunction|StartRoll))))))

(event Custom|Hit
  (bind _startlocation (Variables|Default|GetStartLocation))
  (bind _moveball (Timeline|MoveBall Stop)
    (:Update
      (Transformation|SetWorldLocationAndRotation (Variables|Default|GetDefaultSceneRoot) (Math|Vector|Lerp(Vector) _startlocation (+ _startlocation (Variables|Default|GetTargetLocation)) _moveball) (Math|Rotator|Lerp(Rotator) "0, 0, 0" "360.000000,0.000000,0.000000" _moveball) false false))
    (:Finished
      ;[1 1 1] Reset Ball
      (Transformation|SetWorldLocation (Variables|Default|GetDefaultSceneRoot) (Variables|Default|GetStartLocation) false false)
      (Utilities|FlowControl|Delay (Variables|Default|GetWaitTime))
      (CallFunction|StartRoll))))

(event Custom|StartRoll
  (bind _startlocation (Variables|Default|GetStartLocation))
  ;[1 1 1] Ball rolling animation
  (Components|Animation|PlayAnimation 0 0 0.0 99
    (:then
      (Components|StaticMesh|SetStaticMesh (Variables|Default|GetBallMesh) (.OutItem (Utilities|Array|Random (Variables|Default|GetBallMeshes))))
      (Components|Timeline|SetPlayRate (Variables|Default|GetMoveBall) (Variables|Default|GetPlayRate))
      (bind _moveball (Timeline|MoveBall PlayFromStart)
        (:Update
          (Transformation|SetWorldLocationAndRotation (Variables|Default|GetDefaultSceneRoot) (Math|Vector|Lerp(Vector) _startlocation (+ _startlocation (Variables|Default|GetTargetLocation)) _moveball) (Math|Rotator|Lerp(Rotator) "0, 0, 0" "360.000000,0.000000,0.000000" _moveball) false false))
        (:Finished
          ;[1 1 1] Reset Ball
          (Transformation|SetWorldLocation (Variables|Default|GetDefaultSceneRoot) (Variables|Default|GetStartLocation) false false)
          (Utilities|FlowControl|Delay (Variables|Default|GetWaitTime))
          (CallFunction|StartRoll))))))

(event EventBeginPlay
  ;[1 1 1] Begin Play
  (Variables|Default|SetStartLocation (Transformation|GetActorLocation))
  (CallFunction|StartRoll))

(fn ConstructionScript)