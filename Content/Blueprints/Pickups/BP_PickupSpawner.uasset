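; BP_PickupSpawner is a spawner actor that places a pickup at its spawn point on BeginPlay and respawns one after it is taken.
; It spawns either a fixed item or a random entry from a list of potential items.
; Spawned BP_PickupBase actors get a back-reference to the spawner.
; PickupTaken plays a sound, clears the stored item and starts a one-shot respawn timer.
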(event Custom|SpawnItem
  (bind _returnvalue (Game|SpawnActorfromClass (select (Variables|Default|GetRandomItem?) (.OutItem (Utilities|Array|Random (Variables|Default|GetAllPotentialItems))) (Variables|Default|GetItemToSpawn)) (Transformation|GetWorldTransform (Variables|Default|GetSpawnpoint)) "AlwaysSpawn" 0 0))
  (bind _output_get (Variables|Default|SetSpawnedItem _returnvalue))
  (bind _asbp_pickup_base (Utilities|Casting|CastToBP_PickupBase _output_get))
  (Utilities|IsValid _asbp_pickup_base
    (:Is%20Valid
      (Variables|/Game/Blueprints/Pickups/BP_PickupBase.BP_PickupBase_C|SetSpawnerRef _asbp_pickup_base self))))

(event Custom|StartTimer
  (Utilities|Time|SetTimerbyEvent (delegate Custom|SpawnItem) (Variables|Default|GetTimeToRespawn)))

(event Custom|PickupTaken
  (Audio|PlaySoundatLocation "/Game/Audio/SFX/Obsticles/Pickup_SFX.Pickup_SFX" (Transformation|GetActorLocation) "0, 0, 0" 1.0 1.0 0.0 "/Game/Audio/SoundAttenuation.SoundAttenuation" 0 0 0)
  (Variables|Default|SetSpawnedItem 0)
  (CallFunction|StartTimer))

(event EventBeginPlay
  (CallFunction|SpawnItem))

(fn ConstructionScript)