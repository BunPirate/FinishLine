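; BP_BoostPickup is a pickup that boosts the speed and acceleration of actors overlapping its Box.
; On overlap it calls GetPlayerMessage on the other actor and multiplies the returned object's Speed and Acceleration by SpeedMultiplier.
; The boost is never reverted and the pickup stays in place, so repeat overlaps compound.
; SpeedCheck branches on SpeedBoostActive but does nothing.
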(event OnComponentBeginOverlap(Box)
  (params (OverlappedComponent :type Primitive%20Component%20Object%20Reference) (OtherActor :type Actor%20Object%20Reference) (OtherComp :type Primitive%20Component%20Object%20Reference) (OtherBodyIndex :type Integer) (bFromSweep :type Boolean) (SweepResult :type Hit%20Result%20Structure%20%28by%20ref%29))
  (bind _speedmultiplier (Variables|Default|GetSpeedMultiplier))
  (bind _playerref (Class|BPIPlayer|GetPlayer(Message) OtherActor))
  (Variables|/Game/Blueprints/Player/BP_CustomVehicle.BP_CustomVehicle_C|SetSpeed _playerref (* (Variables|/Game/Blueprints/Player/BP_CustomVehicle.BP_CustomVehicle_C|GetSpeed _playerref) _speedmultiplier))
  (Variables|/Game/Blueprints/Player/BP_CustomVehicle.BP_CustomVehicle_C|SetAcceleration _playerref (* (Variables|/Game/Blueprints/Player/BP_CustomVehicle.BP_CustomVehicle_C|GetAcceleration _playerref) _speedmultiplier)))

(fn ConstructionScript
  (|CallParentFunction))

(fn SpeedCheck
  (if (Variables|Default|GetSpeedBoostActive)
    _))