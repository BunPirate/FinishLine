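; Spline tool that lays two parallel rows of track decals along a path in the construction script.
; It steps the spline by Spacing, offsetting each row sideways by TrackWidth times the spline's Y scale, with yaw following the tangent.
; A downward Visibility trace from the spline centre, not each offset point, sets decal height using the negated actor-relative hit Z, falling back to spline height on a miss.
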(fn ConstructionScript
  (bind _spacing (Variables|Default|GetSpacing))
  (bind _spline (Variables|Default|GetSpline))
  (bind _spacing_2 (Variables|Default|GetSpacing))
  (bind _spline_2 (Variables|Default|GetSpline))
  (for _index (range 0 (Math|Float|Truncate (/ (Spline|GetSplineLength (Variables|Default|GetSpline)) _spacing_2)))
    (bind _outhit (Collision|LineTraceByChannel (Spline|GetLocationatDistanceAlongSpline _spline_2 (* (Math|Conversions|ToFloat(Integer) _index) _spacing_2) "World") (- (Spline|GetLocationatDistanceAlongSpline _spline_2 (* (Math|Conversions|ToFloat(Integer) _index) _spacing_2) "World") "0,0,5000.000000") "TraceTypeQuery1" false 0 "None"))
    (AddComponent|AddDecalComponent false (Math|Transform|MakeTransform (Math|Vector|MakeVector (.X (Class|KismetMathLibrary|BreakVector3f (+ (Spline|GetLocationatDistanceAlongSpline _spline_2 (* (Math|Conversions|ToFloat(Integer) _index) _spacing_2) "Local") (* (Class|SplineComponent|GetRightVectoratDistanceAlongSpline _spline_2 (* (Math|Conversions|ToFloat(Integer) _index) _spacing_2) "Local") (* (Variables|Default|GetTrackWidth) (.y (Class|SplineComponent|GetScaleatDistanceAlongSpline _spline_2 (* (Math|Conversions|ToFloat(Integer) _index) _spacing_2)))))))) (.Y (Class|KismetMathLibrary|BreakVector3f (+ (Spline|GetLocationatDistanceAlongSpline _spline_2 (* (Math|Conversions|ToFloat(Integer) _index) _spacing_2) "Local") (* (Class|SplineComponent|GetRightVectoratDistanceAlongSpline _spline_2 (* (Math|Conversions|ToFloat(Integer) _index) _spacing_2) "Local") (* (Variables|Default|GetTrackWidth) (.y (Class|SplineComponent|GetScaleatDistanceAlongSpline _spline_2 (* (Math|Conversions|ToFloat(Integer) _index) _spacing_2)))))))) (Math|Float|SelectFloat (* (.z (.location (Class|KismetMathLibrary|ConvertTransformtoRelative (Math|Transform|MakeTransform (.Location (Collision|BreakHitResult _outhit))) (Transformation|GetActorTransform)))) -1.0) (.Z (Class|KismetMathLibrary|BreakVector3f (+ (Spline|GetLocationatDistanceAlongSpline _spline_2 (* (Math|Conversions|ToFloat(Integer) _index) _spacing_2) "Local") (* (Class|SplineComponent|GetRightVectoratDistanceAlongSpline _spline_2 (* (Math|Conversions|ToFloat(Integer) _index) _spacing_2) "Local") (* (Variables|Default|GetTrackWidth) (.y (Class|SplineComponent|GetScaleatDistanceAlongSpline _spline_2 (* (Math|Conversions|ToFloat(Integer) _index) _spacing_2)))))))) (.bBlockingHit (Collision|BreakHitResult _outhit)))) (Math|Rotator|MakeRotator 9e+01 9e+01 (.Yaw (Math|Rotator|BreakRotator (Math|Conversions|RotationFromXVector (Spline|GetTangentatDistanceAlongSpline _spline_2 (* (Math|Conversions|ToFloat(Integer) _index) _spacing_2) "Local"))))) "1.000000,1.000000,1.000000")))
  (for _index_2 (range 0 (Math|Float|Truncate (/ (Spline|GetSplineLength (Variables|Default|GetSpline)) _spacing)))
    (bind _outhit_2 (Collision|LineTraceByChannel (Spline|GetLocationatDistanceAlongSpline _spline (* (Math|Conversions|ToFloat(Integer) _index_2) _spacing) "World") (- (Spline|GetLocationatDistanceAlongSpline _spline (* (Math|Conversions|ToFloat(Integer) _index_2) _spacing) "World") "0,0,5000.000000") "TraceTypeQuery1" false 0 "None"))
    (AddComponent|AddDecalComponent false (Math|Transform|MakeTransform (Math|Vector|MakeVector (.X (Class|KismetMathLibrary|BreakVector3f (+ (Spline|GetLocationatDistanceAlongSpline _spline (* (Math|Conversions|ToFloat(Integer) _index_2) _spacing) "Local") (* (Class|SplineComponent|GetRightVectoratDistanceAlongSpline _spline (* (Math|Conversions|ToFloat(Integer) _index_2) _spacing) "Local") (* (* (Variables|Default|GetTrackWidth) -1.0) (.y (Class|SplineComponent|GetScaleatDistanceAlongSpline _spline (* (Math|Conversions|ToFloat(Integer) _index_2) _spacing)))))))) (.Y (Class|KismetMathLibrary|BreakVector3f (+ (Spline|GetLocationatDistanceAlongSpline _spline (* (Math|Conversions|ToFloat(Integer) _index_2) _spacing) "Local") (* (Class|SplineComponent|GetRightVectoratDistanceAlongSpline _spline (* (Math|Conversions|ToFloat(Integer) _index_2) _spacing) "Local") (* (* (Variables|Default|GetTrackWidth) -1.0) (.y (Class|SplineComponent|GetScaleatDistanceAlongSpline _spline (* (Math|Conversions|ToFloat(Integer) _index_2) _spacing)))))))) (Math|Float|SelectFloat (* (.z (.location (Class|KismetMathLibrary|ConvertTransformtoRelative (Math|Transform|MakeTransform (.Location (Collision|BreakHitResult _outhit_2))) (Transformation|GetActorTransform)))) -1.0) (.Z (Class|KismetMathLibrary|BreakVector3f (+ (Spline|GetLocationatDistanceAlongSpline _spline (* (Math|Conversions|ToFloat(Integer) _index_2) _spacing) "Local") (* (Class|SplineComponent|GetRightVectoratDistanceAlongSpline _spline (* (Math|Conversions|ToFloat(Integer) _index_2) _spacing) "Local") (* (* (Variables|Default|GetTrackWidth) -1.0) (.y (Class|SplineComponent|GetScaleatDistanceAlongSpline _spline (* (Math|Conversions|ToFloat(Integer) _index_2) _spacing)))))))) (.bBlockingHit (Collision|BreakHitResult _outhit_2)))) (Math|Rotator|MakeRotator 9e+01 9e+01 (.Yaw (Math|Rotator|BreakRotator (Math|Conversions|RotationFromXVector (Spline|GetTangentatDistanceAlongSpline _spline (* (Math|Conversions|ToFloat(Integer) _index_2) _spacing) "Local"))))) "1.000000,1.000000,1.000000"))))