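; Editor tool Blueprint that builds a track by deforming a mesh along a spline in the Construction Script.
; It adds one Spline Mesh Component per pair of neighboring points, using their local positions and tangents.
; Each segment takes start and end roll from the spline points, converted to radians, so the track can bank.
; The Regenerate flag resets to false on every construction run.
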(fn ConstructionScript
  (bind _spline (Variables|Default|GetSpline))
  (bind _spline_2 (Variables|Default|GetSpline))
  (bind _returnvalue (Spline|GetNumberOfSplinePoints _spline))
  (Variables|Default|SetRegenerate false)
  (for _index (range 0 (- _returnvalue 1))
    (if (not (== _index (- _returnvalue 1)))
      (bind _returnvalue_2 (AddComponent|AddSplineMeshComponent false))
      (Components|StaticMesh|SetStaticMesh _returnvalue_2 (Variables|Default|GetMesh))
      (SplineMesh|SetStartandEnd _returnvalue_2 (Spline|GetLocationatSplinePoint _spline_2 _index "Local") (Spline|GetTangentatSplinePoint _spline_2 _index "Local") (Spline|GetLocationatSplinePoint _spline_2 (+ _index 1) "Local") (Spline|GetTangentatSplinePoint _spline_2 (+ _index 1) "Local") false :!class /Script/Engine.SplineMeshComponent)
      (Class|SplineMeshComponent|SetStartRoll _returnvalue_2 (Math|Float|MultiplybyPi (/ (Spline|GetRollatSplinePoint _spline_2 _index "Local") 1.8e+02)) false)
      (Class|SplineMeshComponent|SetEndRoll _returnvalue_2 (Math|Float|MultiplybyPi (/ (Spline|GetRollatSplinePoint _spline_2 (+ _index 1) "Local") 1.8e+02)) true))))