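; BP_Checkpoint is a trigger volume that registers itself as the player's checkpoint on overlap.
; The overlapping actor's PlayerMessage object receives the checkpoint and, when HalfwayPoint is set, a halfway notification, with a debug "Checkpoint" print.
; Spawn points are gathered from its Arrow components at BeginPlay, and the construction script sizes the box from the BoxExtent variable.
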(event OnComponentBeginOverlap(Box)
  (params (OverlappedComponent :type Primitive%20Component%20Object%20Reference) (OtherActor :type Actor%20Object%20Reference) (OtherComp :type Primitive%20Component%20Object%20Reference) (OtherBodyIndex :type Integer) (bFromSweep :type Boolean) (SweepResult :type Hit%20Result%20Structure%20%28by%20ref%29))
  ;[1 1 1] On overlap, sets the player checkpoint
  (bind _playerref (Class|BPIPlayer|GetPlayer(Message) OtherActor))
  (Utilities|IsValid _playerref
    (:Is%20Valid
      (Default|SetCheckpoint _playerref self)
      (Development|PrintString "Checkpoint" true true "(R=0.141402,G=1.000000,B=0.000000,A=1.000000)")
      ;[1 1 1] Tell player they've reached the halfway point
      (if (Variables|Default|GetHalfwayPoint)
        (Default|ReachedHalfwayPoint _playerref)))))

(event EventBeginPlay
  (Variables|Default|SetSpawnpoints (Actor|GetComponentsByClass "/Script/Engine.ArrowComponent")))

(fn ConstructionScript
  (Components|Box|SetBoxExtent (Variables|Default|GetBox) (Variables|Default|GetBox%20Extent) true))