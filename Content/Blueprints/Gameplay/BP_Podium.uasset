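; BP_Podium is the race podium actor that places finishing vehicles by their position.
; Its TPToPosition event disables the vehicle's input and destroys vehicles ranked fourth or lower.
; Otherwise it zeroes the Body's linear velocity and teleports the vehicle to the transform of the matching first, second or third place component.
; Disconnected leftover nodes for throttle, handbrake and co-op player removal never run.
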(event Custom|TPToPosition
  (params (Position :type Integer) (VehiclePawn :type BP%20Custom%20Vehicle%20Object%20Reference))
  (bind _3rdposition (Variables|Default|Get3rdPosition))
  (bind _2stposition (Variables|Default|Get2stPosition))
  (bind _1stposition (Variables|Default|Get1stPosition))
  (bind _returnvalue (Utilities|Select :Index Position :Option%200 0 :Option%201 _1stposition :Option%202 _2stposition :Option%203 _3rdposition))
  (bind _returnvalue_2 (Transformation|GetWorldTransform _returnvalue))
  (Variables|/Game/Blueprints/Player/BP_CustomVehicle.BP_CustomVehicle_C|SetInputEnabled VehiclePawn false)
  (if (>= Position 4)
    (Actor|DestroyActor VehiclePawn)
    (else
      (Physics|SetPhysicsLinearVelocity (Variables|/Game/Blueprints/Player/BP_CustomVehicle.BP_CustomVehicle_C|GetBody VehiclePawn) "0, 0, 0" false "None")
      (Transformation|SetActorLocationAndRotation VehiclePawn (.location _returnvalue_2) (.rotation _returnvalue_2) false true))))

(fn ConstructionScript)