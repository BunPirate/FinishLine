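; Race game mode for local multiplayer that runs a race from start countdown to win cutscene, then returns to the main menu.
; BeginPlay creates local players from the game instance count, fills remaining slots with AI vehicles and creates a shared HUD.
; SpawnVehicle gives controllers vehicles at PlayerStarts, with input enabled after the countdown.
; Finishers teleport to the podium; the first starts an end timer, and its expiry or everyone finishing triggers the cutscene.
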(event Custom|SpawnAIVehicle
  ;[1 1 1] Spawn a vehicle with no player to get auto possessed by AI
  (bind _returnvalue (Game|SpawnActorfromClass "/Game/Blueprints/Player/BP_CustomVehicle.BP_CustomVehicle_C" (Transformation|GetActorTransform (Utilities|Array|Get(acopy) (Variables|Default|GetSpawnPoints))) "AdjustIfPossibleButAlwaysSpawn" 0 0))
  ;;[1 1 1] Remove the spawnpoint from the array
  (Utilities|Array|RemoveIndex (Variables|Default|GetSpawnPoints))
  (Utilities|Array|Add (Variables|Default|GetVehiclePawnsInRace) _returnvalue))

(event Custom|SetupPlayers
  (params (NumberOfPlayers :type Integer))
  ;[1 1 1] Get all spawnpoints
  (bind _outactors (Actor|GetAllActorsOfClass "/Script/Engine.PlayerStart"))
  (Variables|Default|SetSpawnPoints _outactors)
  ;[1 1 1] Add additional players if needed
  (for _index (range 0 (- NumberOfPlayers 1))
    (Class|GameplayStatics|CreatePlayer _index))
  (for _index_2 (range 0 (Utilities|Operators|Subtract (Variables|Default|GetBotFillPlayerCount) NumberOfPlayers 1))
    (CallFunction|SpawnAIVehicle)))

(event Custom|RaceStartTimer
  (bind _secondsleft (Variables|Default|GetSecondsLeft))
  ;[1 1 1] Repeated every second of race start timer
  (Default|SetCountdownNum (Variables|Default|GetMainHUD) (Utilities|Text|ToText(Integer) (Variables|Default|GetSecondsLeft)))
  (Math|Integer|DecrementInt _secondsleft
    (:%20%20
      (if (<= _secondsleft -1)
        (Utilities|Time|ClearandInvalidateTimerbyHandle (Variables|Default|GetRaceStartTimerHandle))
        (Default|SetCountdownNum (Variables|Default|GetMainHUD) "RACE!")
        (for _array_element (Variables|Default|GetVehiclePawnsInRace)
          (Variables|/Game/Blueprints/Player/BP_CustomVehicle.BP_CustomVehicle_C|SetInputEnabled _array_element true))))))

(event Custom|OnStopSequence
  ;[1 1 1] All players finished
  (Game|OpenLevel(byObjectReference) "/Game/Levels/Final/L_MainMenu.L_MainMenu"))

(event Custom|PlayerFinished
  (params (Vehicle :type BP%20Custom%20Vehicle%20Object%20Reference))
  (bind _playersfinished (Variables|Default|GetPlayersFinished))
  ;[1 1 1] Gets called when a player finishes the race
  (Utilities|Array|RemoveItem (Variables|Default|GetVehiclePawnsInRace) Vehicle)
  (bind _result (Math|Integer|IncrementInt _playersfinished)
    (:%20%20
      (Default|TPtoPosition (Variables|Default|GetPodiumRef) _result Vehicle)
      (CallFunction|StartGameEndCountdown)
      (if (>= _playersfinished (Variables|Default|GetBotFillPlayerCount))
        ;[1 1 1] All players finished
        (for _array_element (Variables|Default|GetPlayerControllers)
          (if (!= _array_element (Game|GetPlayerController 0))
            (bind _asplayer_controller (Utilities|Casting|CastToPlayerController _array_element))
            (Class|GameplayStatics|RemovePlayer _asplayer_controller false)))
        (bind _returnvalue (Sequencer|Player|CreateLevelSequencePlayer "/Game/Levels/WinCutscene.WinCutscene" (Utilities|Struct|MakeMovieSceneSequencePlaybackSettings true "(Value=0)")))
        (EventDispatchers|BindEventtoOnStop _returnvalue (delegate Custom|OnStopSequence))))))

(event Custom|StartGameEndCountdown
  ;[1 1 1] Begin end game timer when one player finishes race
  (Utilities|FlowControl|DoOnce false
    (:Completed
      (bind _returnvalue (Utilities|Time|SetTimerbyEvent (delegate Custom|AddToEndTimer) 1.0 true))
      (Variables|Default|SetGameEndTimerHandle _returnvalue))))

(event Custom|AddToEndTimer
  ;[1 1 1] Begin end game timer when one player finishes race
  (Default|SetEndGameCountdownNum (Variables|Default|GetMainHUD) (Utilities|Text|ToText(Integer) (Variables|Default|GetGameEndTimer)))
  (if (<= (Variables|Default|GetGameEndTimer) 0)
    (Utilities|Time|ClearandInvalidateTimerbyHandle (Variables|Default|GetGameEndTimerHandle))
    (Default|SetEndGameCountdownNum (Variables|Default|GetMainHUD) "GAME OVER!")
    ;[1 1 1] All players finished
    (for _array_element (Variables|Default|GetPlayerControllers)
      (if (!= _array_element (Game|GetPlayerController 0))
        (bind _asplayer_controller (Utilities|Casting|CastToPlayerController _array_element))
        (Class|GameplayStatics|RemovePlayer _asplayer_controller false)))
    (bind _returnvalue (Sequencer|Player|CreateLevelSequencePlayer "/Game/Levels/WinCutscene.WinCutscene" (Utilities|Struct|MakeMovieSceneSequencePlaybackSettings true "(Value=0)")))
    (EventDispatchers|BindEventtoOnStop _returnvalue (delegate Custom|OnStopSequence))
    (else
      (Math|Integer|DecrementInt (Variables|Default|GetGameEndTimer)))))

(event EventBeginPlay
  ;[1 1 1] Gets number of players from game inst
  (bind _asbp_game_instance (Utilities|Casting|CastToBP_GameInstance (Game|GetGameInstance)))
  (bind _returnvalue (Actor|GetActorOfClass "/Game/Blueprints/Gamemode/BP_CoopPlayerController.BP_CoopPlayerController_C"))
  (Class|GameplayStatics|RemovePlayer _returnvalue true)
  (CallFunction|SetupPlayers (Variables|/Game/Blueprints/Gamemode/BP_GameInstance.BP_GameInstance_C|GetNumOfPlayers _asbp_game_instance))
  (bind _returnvalue_2 (Actor|GetActorOfClass "/Game/Blueprints/Gameplay/BP_Podium.BP_Podium_C"))
  (Variables|Default|SetPodiumRef _returnvalue_2)
  ;[1 1 1] Create HUD for whole screen
  (bind _returnvalue_3 (UserInterface|CreateWidget "/Game/Blueprints/UI/HUD/W_HUDMain.W_HUDMain_C"))
  (UserInterface|Viewport|AddtoViewport _returnvalue_3 0)
  (Variables|Default|SetMainHUD _returnvalue_3)
  (bind _returnvalue_4 (Utilities|Time|SetTimerbyEvent (delegate Custom|RaceStartTimer) 1.0 true))
  (Variables|Default|SetRaceStartTimerHandle _returnvalue_4)
  (if (Class|KismetSystemLibrary|IsPackagedforDistribution)
    (Development|ExecuteConsoleCommand "disableallscreenmessages " 0)))

(fn ConstructionScript)

(fn SpawnVehicle
  (params (PlayerController :type Controller%20Object%20Reference))
  (bind _spawnpoints (Variables|Default|GetSpawnPoints))
  (bind _output (Utilities|Array|Get(acopy) _spawnpoints))
  (bind _returnvalue (Transformation|GetActorTransform _output))
  ;[1 1 1] Spawn a vehicle for the player controller
  (Utilities|Array|Add (Variables|Default|GetPlayerControllers) PlayerController)
  (bind _returnvalue_2 (AI|SpawnAIFromClass "/Game/Blueprints/Player/BP_CustomVehicle.BP_CustomVehicle_C" 0 (.location _returnvalue) (.rotation _returnvalue) false 0))
  (bind _playerref (Class|BPIPlayer|GetPlayer(Message) _returnvalue_2))
  (Utilities|Array|RemoveIndex (Variables|Default|GetSpawnPoints))
  ;;[1 1 1] Remove the spawnpoint from the array
  (Utilities|Array|Add (Variables|Default|GetVehiclePawnsInRace) _playerref)
  (Pawn|Possess PlayerController _playerref)
  (return _playerref))

(fn GetGamemode
  (return self))