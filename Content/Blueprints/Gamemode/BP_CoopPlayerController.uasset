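; Player controller for co-op racing that has BP_RaceGamemode spawn its vehicle on BeginPlay and keeps it as PlayerRef.
; Forwards driving, air control, drift, item, weapon, camera, respawn and boostpad inputs to that vehicle; fire and drift also request cutscene skips.
; InitController creates a per-player HUD and links it to the vehicle.
; FlipFlops toggle the debug and pause menus, with pause input mode applied to player 0.
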(event Custom|InitController
  (bind _playerref (Variables|Default|GetPlayerRef))
  ;[1 1 1] After a delay create individual player widget
  (bind _returnvalue (UserInterface|CreateWidget "/Game/Blueprints/UI/HUD/W_HUDPlayer.W_HUDPlayer_C" self))
  (UserInterface|Viewport|AddtoPlayerScreen _returnvalue)
  (bind _output_get (Variables|Default|SetPlayerHUD _returnvalue))
  (bind _output_get_2 (Variables|/Game/Blueprints/Player/BP_CustomVehicle.BP_CustomVehicle_C|SetHudRef _playerref _output_get))
  (Default|InitialisePlayerHUD _output_get self)
  (Default|UpdateInventory _playerref))

(event Custom|SkipCutsceneEvent
  (bind _gamemoderef (Class|BPIGamemode|GetGamemode(Message) (Game|GetGameMode)))
  (Utilities|IsValid _gamemoderef
    (:Is%20Valid
      (Default|SkipCutscene _gamemoderef))))

(event EventBeginPlay
  (Variables|Default|SetbShowMouseCursor false)
  (bind _asbp_race_gamemode (Utilities|Casting|CastToBP_RaceGamemode (Game|GetGameMode)))
  (bind _playerref (Default|SpawnVehicle _asbp_race_gamemode self))
  (Variables|Default|SetPlayerRef _playerref))

(event Input|ActionEvents|InputActionFireWeapon
  (params (Key :type Key%20Structure :default "None"))
  (bind _playerref (Variables|Default|GetPlayerRef))
  ;[0.0612 1 0] Inputs
  (:Pressed
    (Default|FireWeaponPressed _playerref)
    (CallFunction|SkipCutsceneEvent))
  (:Released
    (Default|FireWeaponReleased _playerref)))

(event Input|ActionEvents|InputActionSwitchCamera
  (params (Key :type Key%20Structure :default "None"))
  (bind _playerref (Variables|Default|GetPlayerRef))
  ;[0.0612 1 0] Inputs
  (:Pressed
    (Default|FlipCamera _playerref))
  (:Released
    (Default|UnFlipCamera _playerref)))

(event Input|ActionEvents|InputActionUseItem
  (params (Key :type Key%20Structure :default "None"))
  (bind _playerref (Variables|Default|GetPlayerRef))
  (:Pressed
    (Default|StartUseItem _playerref))
  (:Released
    (Default|EndUseItem _playerref)))

(event Input|ActionEvents|InputActionSwapItem
  (params (Key :type Key%20Structure :default "None"))
  (:Pressed
    (Default|SwapItem (Variables|Default|GetPlayerRef))))

(event Input|ActionEvents|InputActionDrift
  (params (Key :type Key%20Structure :default "None"))
  (bind _playerref (Variables|Default|GetPlayerRef))
  ;[0.0612 1 0] Inputs
  (:Pressed
    (Default|StartDrift _playerref)
    (CallFunction|SkipCutsceneEvent))
  (:Released
    (Default|EndDrift _playerref)))

(event Input|ActionEvents|InputActionPause
  (params (Key :type Key%20Structure :default "None"))
  (bind _returnvalue (Game|GetPlayerController 0))
  (bind _returnvalue_2 (Game|GetPlayerController 0))
  ;[0.0612 1 0] Inputs
  ;;[1 1 1] Pause Game
  (:Pressed
    (Utilities|FlowControl|FlipFlop
      (:A
        (bind _returnvalue_3 (UserInterface|CreateWidget "/Game/Blueprints/MainMenu/W_PauseMenu.W_PauseMenu_C"))
        (UserInterface|Viewport|AddtoViewport _returnvalue_3 0)
        (Game|SetGamePaused true)
        (Input|SetInputModeGameandUI _returnvalue 0 "DoNotLock" true)
        (Variables|/Script/Engine.PlayerController|SetbShowMouseCursor _returnvalue true))
      (:B
        (Widget|RemovefromParent _returnvalue_3)
        (Input|SetInputModeGameOnly _returnvalue_2)
        (Variables|/Script/Engine.PlayerController|SetbShowMouseCursor _returnvalue_2 true)
        (Game|SetGamePaused false)))))

(event Input|ActionEvents|InputActionRespawn
  (params (Key :type Key%20Structure :default "None"))
  (bind _playerref (Variables|Default|GetPlayerRef))
  (:Pressed
    (if (Variables|/Game/Blueprints/Player/BP_CustomVehicle.BP_CustomVehicle_C|GetCanRespawn? _playerref)
      (Default|RespawnatLastCheckpoint _playerref)
      (Variables|/Game/Blueprints/Player/BP_CustomVehicle.BP_CustomVehicle_C|SetCanRespawn? _playerref false))))

(event Input|ActionEvents|InputActionRetrieveBoostpads
  (params (Key :type Key%20Structure :default "None"))
  (bind _playerref (Variables|Default|GetPlayerRef))
  ;[0.0612 1 0] Inputs
  (:Pressed
    (Utilities|IsValid _playerref
      (:Is%20Valid
        (Default|RetrieveBoostpads _playerref)))))

(event Input|AxisEvents|InputAxisLookUp
  (params (AxisValue :type Float%20%28single-precision%29))
  (if (or (> AxisValue 0.1) (< AxisValue -0.9))
    (Default|AirControlVertical (Variables|Default|GetPlayerRef) AxisValue)))

(event Input|AxisEvents|InputAxisMoveRight
  (params (AxisValue :type Float%20%28single-precision%29))
  (bind _playerref (Variables|Default|GetPlayerRef))
  ;[0.0612 1 0] Inputs
  (Default|MoveRight _playerref AxisValue)
  (if (or (> AxisValue 0.1) (< AxisValue -0.9))
    (Variables|/Game/Blueprints/Player/BP_CustomVehicle.BP_CustomVehicle_C|SetSteeringAxis _playerref AxisValue)))

(event Input|AxisEvents|InputAxisLookRight
  (params (AxisValue :type Float%20%28single-precision%29))
  (if (or (> AxisValue 0.1) (< AxisValue -0.9))
    (Default|AirControlHorizontal (Variables|Default|GetPlayerRef) AxisValue)))

(event Input|AxisEvents|InputAxisMoveForward
  (params (AxisValue :type Float%20%28single-precision%29))
  ;[0.0612 1 0] Inputs
  (Default|MoveForward (Variables|Default|GetPlayerRef) AxisValue))

(event Input|KeyboardEvents|Home
  (params (Key :type Key%20Structure :default "None"))
  ;[1 1 1] Debug
  (:Pressed
    (Utilities|FlowControl|FlipFlop
      (:A
        (bind _returnvalue (UserInterface|CreateWidget "/Game/Blueprints/UI/HUD/W_DebugMenu.W_DebugMenu_C"))
        (UserInterface|Viewport|AddtoViewport _returnvalue 0)
        (Variables|Default|SetDebugMenu _returnvalue)
        (Variables|Default|SetbShowMouseCursor true))
      (:B
        (Widget|RemovefromParent (Variables|Default|GetDebugMenu))
        (Variables|Default|SetbShowMouseCursor false)))))

(fn ConstructionScript)