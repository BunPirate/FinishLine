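; Track editor tool that places copies of a chosen mesh along a spline at a set spacing.
; The construction script fills an instanced static mesh component, orienting each instance along the spline tangent.
; With StickToGround on, a downward visibility trace from each point supplies the height, converted to actor-relative space, falling back to spline height when nothing is hit.
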(event EventBeginPlay)

(event Collision|EventActorBeginOverlap
  (params (OtherActor :type Actor%20Object%20Reference)))

(event EventTick
  (params (DeltaSeconds :type Float%20%28single-precision%29)))

(fn ConstructionScript
  (bind _spacing (Variables|Default|GetSpacing))
  (bind _spline (Variables|Default|GetSpline))
  (Components|StaticMesh|SetStaticMesh (Variables|Default|GetInstancedStaticMesh) (Variables|Default|GetMesh))
  (for _index (range 0 (Math|Float|Truncate (/ (Spline|GetSplineLength (Variables|Default|GetSpline)) _spacing)))
    (if (Variables|Default|GetStickToGround)
      (bind _outhit (Collision|LineTraceByChannel (Spline|GetLocationatDistanceAlongSpline _spline (* (Math|Conversions|ToFloat(Integer) _index) _spacing) "World") (- (Spline|GetLocationatDistanceAlongSpline _spline (* (Math|Conversions|ToFloat(Integer) _index) _spacing) "World") "0,0,5000.000000") "TraceTypeQuery1" false 0 "None"))
      (Components|InstancedStaticMesh|AddInstance (Variables|Default|GetInstancedStaticMesh) (Math|Transform|MakeTransform (Math|Vector|MakeVector (.X (Class|KismetMathLibrary|BreakVector3f (Spline|GetLocationatDistanceAlongSpline _spline (* (Math|Conversions|ToFloat(Integer) _index) _spacing) "Local"))) (.Y (Class|KismetMathLibrary|BreakVector3f (Spline|GetLocationatDistanceAlongSpline _spline (* (Math|Conversions|ToFloat(Integer) _index) _spacing) "Local"))) (Math|Float|SelectFloat (* (.z (.location (Class|KismetMathLibrary|ConvertTransformtoRelative (Math|Transform|MakeTransform (.Location (Collision|BreakHitResult _outhit)) "0,0.000000, 0") (Transformation|GetActorTransform)))) -1.0) (.Z (Class|KismetMathLibrary|BreakVector3f (Spline|GetLocationatDistanceAlongSpline _spline (* (Math|Conversions|ToFloat(Integer) _index) _spacing) "Local"))) (.bBlockingHit (Collision|BreakHitResult _outhit)))) (Math|Conversions|RotationFromXVector (Spline|GetTangentatDistanceAlongSpline _spline (* (Math|Conversions|ToFloat(Integer) _index) _spacing) "Local")) "1.000000,1.000000,1.000000") false)
      (else
        (Components|InstancedStaticMesh|AddInstance (Variables|Default|GetInstancedStaticMesh) (Math|Transform|MakeTransform (Spline|GetLocationatDistanceAlongSpline _spline (* (Math|Conversions|ToFloat(Integer) _index) _spacing) "Local") (Math|Conversions|RotationFromXVector (Spline|GetTangentatDistanceAlongSpline _spline (* (Math|Conversions|ToFloat(Integer) _index) _spacing) "Local")) "1.000000,1.000000,1.000000") false)))))