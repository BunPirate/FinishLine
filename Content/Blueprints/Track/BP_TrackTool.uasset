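; BP_TrackTool is a track-building Blueprint that lays spline mesh segments along its Spline component.
; The Construction Script adds one SplineMeshComponent for each pair of consecutive spline points, skipping the last point.
; Each segment takes its start and end positions and tangents from those points in local space, and its index is printed for debugging.
; A disconnected world-space loop that sets end position and tangent never runs.
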(fn ConstructionScript
  (bind _spline (Variables|Default|GetSpline))
  (bind _spline_2 (Variables|Default|GetSpline))
  (bind _returnvalue (Spline|GetNumberOfSplinePoints _spline))
  (for _index (range 0 (- _returnvalue 1))
    (if (not (== _index (- _returnvalue 1)))
      (bind _returnvalue_2 (AddComponent|AddSplineMeshComponent false))
      (Development|PrintString (Utilities|String|ToString(Integer) _index))
      (SplineMesh|SetStartandEnd _returnvalue_2 (Spline|GetLocationatSplinePoint _spline_2 _index "Local") (Spline|GetTangentatSplinePoint _spline_2 _index "Local") (Spline|GetLocationatSplinePoint _spline_2 (+ _index 1) "Local") (Spline|GetTangentatSplinePoint _spline_2 (+ _index 1) "Local") true :!class /Script/Engine.SplineMeshComponent))))