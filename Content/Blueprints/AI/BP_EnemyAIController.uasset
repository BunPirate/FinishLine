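; AI controller for enemy racers that drives its pawn along the first BP_AIPath spline in the level.
; A staggered looping timer steers toward a look-ahead spline point, easing throttle on sharp turns, or reverses with full steer when a forward sphere trace hits world-static geometry.
; Tick applies these inputs and fires the weapon while the pawn is slipstreaming.
; A second timer respawns the pawn at its last checkpoint when allowed.
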(event Custom|AIUpdate
  (bind _aipaths (Variables|Default|GetAIPaths))
  (bind _pawnref (Variables|Default|GetPawnRef))
  (bind _pawnref_2 (Variables|Default|GetPawnRef))
  (bind _pawnref_3 (Variables|Default|GetPawnRef))
  (bind _returnvalue (Transformation|GetActorLocation _pawnref_2))
  (bind _returnvalue_2 (Transformation|GetActorRotation _pawnref_3))
  (bind _output (Utilities|Array|Get(acopy) _aipaths))
  (bind _firepoint (Variables|/Game/Blueprints/Player/BP_CustomVehicle.BP_CustomVehicle_C|GetFirePoint _pawnref))
  (bind _returnvalue_3 (Transformation|GetWorldLocation _firepoint))
  (bind _spline (Variables|/Game/Blueprints/AI/BP_AIPath.BP_AIPath_C|GetSpline _output))
  (bind _returnvalue_4 (Class|SplineComponent|FindTangentClosesttoWorldLocation _spline _returnvalue "World"))
  (bind _returnvalue_5 (Math|Vector|Normalize _returnvalue_4))
  (bind _returnvalue_6 (* _returnvalue_5 2e+03))
  (bind _returnvalue_7 (+ _returnvalue_6 _returnvalue))
  (bind _returnvalue_8 (Spline|FindLocationClosesttoWorldLocation _spline _returnvalue_7 "World"))
  (bind _returnvalue_9 (Math|Rotator|FindLookatRotation _returnvalue _returnvalue_8))
  (bind _returnvalue_10 (Math|Rotator|Delta(Rotator) _returnvalue_9 _returnvalue_2))
  (bind _returnvalue_11 (Math|Float|MapRangeClamped (.yaw _returnvalue_10) -9e+01 9e+01 -1.0 1.0))
  (bind _outhit (Collision|SphereTraceForObjects _returnvalue_3 (+ _returnvalue_3 (* (Math|Vector|GetForwardVector _firepoint) 5e+02)) 25.0 (Utilities|Array|MakeArray "ObjectTypeQuery1") false 0 "None"))
  (if (.bBlockingHit (Collision|BreakHitResult _outhit))
    (Variables|Default|SetSteeringInput 1.0)
    (Variables|Default|SetThrottleInput -1.0)
    (else
      ;[1 1 1] Steer to spline
      (Variables|Default|SetThrottleInput (Math|Float|MapRangeClamped (Math|Float|Absolute(Float) _returnvalue_11) 0.0 1.0 1.0 0.5))
      (Variables|Default|SetSteeringInput (* (Math|Float|MapRangeClamped (Math|Vector|Distance(Vector) _returnvalue_8 _returnvalue) 0.0 1.5e+04 1.0 0.5) _returnvalue_11)))))

(event Custom|TryRespawn
  (bind _pawnref (Variables|Default|GetPawnRef))
  (if (Variables|/Game/Blueprints/Player/BP_CustomVehicle.BP_CustomVehicle_C|GetCanRespawn? _pawnref)
    (Default|RespawnatLastCheckpoint _pawnref)
    (Variables|/Game/Blueprints/Player/BP_CustomVehicle.BP_CustomVehicle_C|SetCanRespawn? _pawnref false)))

(event EventBeginPlay
  (Utilities|FlowControl|Delay 0.01)
  (bind _outactors (Actor|GetAllActorsOfClass "/Game/Blueprints/AI/BP_AIPath.BP_AIPath_C"))
  (Variables|Default|SetAIPaths _outactors)
  (bind _playerref (Class|BPIPlayer|GetPlayer(Message) (Pawn|GetControlledPawn)))
  (bind _output_get (Variables|Default|SetPawnRef _playerref))
  (Utilities|IsValid _output_get
    (:Is%20Valid
      (Utilities|Time|SetTimerbyEvent (delegate Custom|AIUpdate) 0.1 true 1.0 0.5)
      (Utilities|Time|SetTimerbyEvent (delegate Custom|TryRespawn) 1.0 true 5.0))
    (:Is%20Not%20Valid
      (Actor|DestroyActor))))

(event EventTick
  (params (DeltaSeconds :type Float%20%28single-precision%29))
  (bind _pawnref (Variables|Default|GetPawnRef))
  (Utilities|IsValid (Variables|Default|GetPawnRef)
    (:Is%20Valid
      (Default|MoveRight (Variables|Default|GetPawnRef) (Variables|Default|GetSteeringInput))
      (Default|MoveForward _pawnref (Variables|Default|GetThrottleInput))
      (if (Variables|/Game/Blueprints/Player/BP_CustomVehicle.BP_CustomVehicle_C|GetSlipStreaming? _pawnref)
        (Default|FireWeaponPressed _pawnref)
        (else
          (Default|FireWeaponReleased _pawnref))))))

(fn ConstructionScript)