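; Base projectile actor that launches forward on spawn and damages whatever it hits.
; BeginPlay reads its weapon stats row from DT_WeaponStats and applies a velocity-change impulse to its collision using the stat speed.
; On hit it sends a damage message to any actor except its instigator, then plays effects and destroys itself.
; Effects include a burst particle system, plus decal and sound selected by physical surface type.
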(event Custom|HitEffects
  (bind _hit_phys_mat (Variables|Default|GetHit%20Phys%20Mat))
  (bind _surfacetype (Variables|/Script/PhysicsCore.PhysicalMaterial|GetSurfaceType _hit_phys_mat))
  ;[1 1 1] Projectile hit effects
  (Niagara|SpawnSystematLocation "/Niagara/DefaultAssets/Templates/Systems/RadialBurst.RadialBurst" (Transformation|GetActorLocation))
  (Class|GameplayStatics|SpawnDecalAttached (Utilities|Select :Index _surfacetype :SurfaceType_Default 0 :SurfaceType1 "/Game/Materials/M_DecalMaster.M_DecalMaster") "100.000000,100.000000,100.000000" (Variables|/Script/Engine.Actor|GetRootComponent (Variables|Default|GetHitActor)) "None" (Transformation|GetActorLocation) (Math|Conversions|RotationFromXVector (Variables|Default|GetHit%20Normal)) "KeepWorldPosition" 2e+01)
  (Audio|PlaySoundatLocation (Utilities|Select :Index _surfacetype :SurfaceType_Default 0 :SurfaceType1 "/Game/Audio/SFX/Vehicle/VehicleHit3.VehicleHit3") (Transformation|GetActorLocation) "0, 0, 0" 1.0 1.0 0.0 "/Game/Audio/SoundAttenuation.SoundAttenuation" 0 0 0))

(event Collision|EventHit
  (params (MyComp :type Primitive%20Component%20Object%20Reference) (Other :type Actor%20Object%20Reference) (OtherComp :type Primitive%20Component%20Object%20Reference) (bSelfMoved :type Boolean) (HitLocation :type Vector :default "0, 0, 0") (HitNormal :type Vector :default "0, 0, 0") (NormalImpulse :type Vector :default "0, 0, 0") (Hit :type Hit%20Result%20Structure%20%28by%20ref%29))
  (bind _returnvalue (Game|GetInstigator))
  ;[1 1 1] On projectile hit
  (Variables|Default|SetHit%20Normal (.normal Hit))
  (Variables|Default|SetHit%20Phys%20Mat (.physmat Hit))
  (bind _output_get (Variables|Default|SetHitActor Other))
  (if (== _output_get _returnvalue)
    _
    (else
      (Class|BPIDamageable|DoDamage(Message) Other (.Damage (Utilities|Struct|BreakS_WeaponStats (Variables|Default|GetWeaponStats))) _returnvalue)))
  (CallFunction|HitEffects)
  (Actor|DestroyActor))

(event EventBeginPlay
  ;[1 1 1] Send projectile forward
  (bind _returnvalue (Utilities|GetDataTableRow "/Game/Blueprints/Datatables/DT_WeaponStats.DT_WeaponStats" (Variables|Default|GetDatatableRowNumber))
    (:then
      (Variables|Default|SetWeaponStats _returnvalue)
      (Physics|AddImpulse (Variables|Default|GetCollision) (* (Transformation|GetActorForwardVector) (.Speed (Utilities|Struct|BreakS_WeaponStats (Variables|Default|GetWeaponStats)))) "None" true))))

(fn ConstructionScript)